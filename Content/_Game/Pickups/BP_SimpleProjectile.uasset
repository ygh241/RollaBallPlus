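; Simple projectile actor that moves along its forward vector every tick, using a swept world offset scaled by delta time and MoveSpeed.
; BeginPlay caches the starting speed as InitialMoveSpeed.
; SpeedBoost multiplies the current speed, then restores the cached speed after a retriggerable delay.
; Repeated boosts during that delay compound the speed and restart the timer.
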(event EventTick
  (params (DeltaSeconds :type Float%20%28single-precision%29))
  (Transformation|AddActorWorldOffset (* (* DeltaSeconds (Variables|Default|GetMoveSpeed)) (Transformation|GetActorForwardVector)) true))

(event EventSpeedBoost
  (params (Multiplier :type Float%20%28double-precision%29) (Duration :type Float%20%28double-precision%29))
  (Variables|Default|SetMoveSpeed (* Multiplier (Variables|Default|GetMoveSpeed))) ; SpeedUp
  (Utilities|FlowControl|RetriggerableDelay Duration) ; Wait
  (Variables|Default|SetMoveSpeed (Variables|Default|GetInitialMoveSpeed)) ; Reset Speed
)

(event EventBeginPlay
  (Variables|Default|SetInitialMoveSpeed (Variables|Default|GetMoveSpeed)))

(fn ConstructionScript)